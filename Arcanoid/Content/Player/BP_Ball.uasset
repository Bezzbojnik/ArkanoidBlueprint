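; BP_Ball is a bouncing ball actor that strikes BP_Enemy targets.
; Launch sets its travel direction to the actor's forward vector, and Tick moves it along that direction by Speed with a swept world offset.
; On a blocking hit, the direction is reflected around the surface normal.
; The Sphere component's hit event casts the other actor to BP_Enemy and calls HitMe on it.
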(event OnComponentHit(Sphere)
  (params (HitComponent :type Primitive%20Component%20Object%20Reference) (OtherActor :type Actor%20Object%20Reference) (OtherComp :type Primitive%20Component%20Object%20Reference) (NormalImpulse :type Vector :default "0, 0, 0") (Hit :type Hit%20Result%20Structure%20%28by%20ref%29))
  ;[1 1 1] Если сопрекоснется с платформой-целью, вызвать функцию HitMe
  (bind _asbp_enemy (Utilities|Casting|CastToBP_Enemy OtherActor))
  (Default|HitMe _asbp_enemy))

(event Custom|Launch
  (Variables|Default|SetDirection (Transformation|GetActorForwardVector)) ; Направляющий вектор
)

(event EventBeginPlay)

(event EventTick
  (params (DeltaSeconds :type Float%20%28single-precision%29))
  ;[1 1 1] Смещает мячик по направляющему вектору со скоростью speed
  (bind _sweephitresult (Transformation|AddActorWorldOffset (* (Variables|Default|GetDirection) (* DeltaSeconds (Variables|Default|GetSpeed))) true))
  ;[1 1 1] Смена направления в зависимости от угла столкновения с препятствием
  (if (.bBlockingHit (Collision|BreakHitResult _sweephitresult))
    (Variables|Default|SetDirection (Math|Vector|GetReflectionVector (Variables|Default|GetDirection) (.Normal (Collision|BreakHitResult _sweephitresult))))))

(fn ConstructionScript)