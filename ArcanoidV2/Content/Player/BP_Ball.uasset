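; BP_Ball is a bouncing ball that damages BP_Enemy targets and ends the game on touching lava.
; Launch sets its direction from the forward vector, and Tick moves it with a swept offset, reflecting that direction off the surface normal on blocking hits.
; Sphere hits call HitMe on enemies and notify WidgetManager; other hits check for a Lava tag to stop movement and trigger game over, then play alternating sounds.
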(event OnComponentHit(Sphere)
  (params (HitComponent :type Primitive%20Component%20Object%20Reference) (OtherActor :type Actor%20Object%20Reference) (OtherComp :type Primitive%20Component%20Object%20Reference) (NormalImpulse :type Vector :default "0, 0, 0") (Hit :type Hit%20Result%20Structure%20%28by%20ref%29))
  (bind _audio (Variables|Default|GetAudio))
  ;[1 1 1] Если сопрекоснется с платформой-целью, вызвать функцию HitMe
  (bind _asbp_enemy (Utilities|Casting|CastToBP_Enemy OtherActor)
    (:then
      (Default|HitMe _asbp_enemy)
      (Default|HitEnemy (Variables|Default|GetWidgetManager)))
    (:CastFailed
      ;[1 1 1] Если коснулись стенки с тегом "Лава", то игра окончена (на сцене это красный прямоугольник внизу)
      (for _array_element (Variables|/Script/Engine.Actor|GetTags OtherActor)
        (if (Utilities|Name|Equal(Name) _array_element "Lava")
          (Variables|Default|SetStopMove true)
          (Default|GameOver (Variables|Default|GetWidgetManager))))
      ;[1 1 1] Вопроизведение звуков при столкновении со стенами и нашей платформой
      (Utilities|FlowControl|FlipFlop
        (:A
          (Audio|Components|Audio|SetSound _audio "/Game/Audio/bababooey-sound-effect_Cue.bababooey-sound-effect_Cue"))
        (:B
          (Audio|Components|Audio|SetSound _audio "/Game/Audio/brue_Cue.brue_Cue")))
      (Components|Activation|Activate _audio true))))

(event Custom|Launch
  ;[1 1 1] Задаем начальный вектор по оси Х
  (Variables|Default|SetDirection (Transformation|GetActorForwardVector)) ; Направляющий вектор
)

(event EventBeginPlay)

(event EventTick
  (params (DeltaSeconds :type Float%20%28single-precision%29))
  ;[1 1 1] Смещает мячик по направляющему вектору со скоростью speed
  (if (not (Variables|Default|GetStopMove))
    (bind _sweephitresult (Transformation|AddActorWorldOffset (* (Variables|Default|GetDirection) (* DeltaSeconds (Variables|Default|GetSpeed))) true))
    ;[1 1 1] Смена направления в зависимости от угла столкновения с препятствием
    (if (.bBlockingHit (Collision|BreakHitResult _sweephitresult))
      (Variables|Default|SetDirection (Math|Vector|GetReflectionVector (Variables|Default|GetDirection) (.Normal (Collision|BreakHitResult _sweephitresult)))))))

(fn ConstructionScript)